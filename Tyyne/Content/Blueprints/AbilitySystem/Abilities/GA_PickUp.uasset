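; Gameplay ability that lets the player pick up an interactable item into the inventory.
; On activation it commits, casts player 0's pawn to AuroraCharacter and uses that character's interactable trace to find the target.
; A valid target goes to the inventory component, and a successful add fires the character's inventory change dispatcher.
; Any failed step after the commit prints a debug message, and the ability then ends.
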(event `self.K2_ActivateAbility`
  (`self.K2_CommitAbility`)
  (bind _asaurora_character (cast `/Game/Blueprints/AuroraCharacter` (`GameplayStatics.GetPlayerPawn` 0))
    (:`then`
      (bind _hititem (`/Game/Blueprints/AuroraCharacter.InteractableTrace` _asaurora_character))
      (`/Engine/EditorBlueprintResources/StandardMacros.IsValid` _hititem
        (:`Is Valid`
          (bind _returnvalue (`InventoryComponent.AddItemToInventory` (`TyyneCharacter.GetInventoryComponent` _asaurora_character) _hititem))
          (if _returnvalue
            (`/Game/Blueprints/AuroraCharacter.InventoryChangeDispatcher` _asaurora_character)
            (else
              (`KismetSystemLibrary.PrintString` "Not Valid" :!label _label))))
        (:`Is Not Valid`
          (goto _label))))
    (:`CastFailed`
      (goto _label)))
  (`self.K2_EndAbility`))