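; BP_Door is an interactable door prop that swings open or closed when interacted with.
; Interact calls ToggleDoor and returns true, and a FlipFlop alternates between playing and reversing the DoorToggle timeline.
; The timeline's Angle track drives the relative yaw of DoorMesh, and IsOpen flips when the timeline finishes.
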(event `ToggleDoor`
  (`/Engine/EditorBlueprintResources/StandardMacros.FlipFlop`
    (:`A`
      (bind (_direction _angle) (`Timeline|DoorToggle` :!label _label)
        (:`Update`
          (`SceneComponent.K2_SetRelativeRotation` (`self.DoorMesh`) (`KismetMathLibrary.MakeRotator` 0.0 0.0 _angle) false false))
        (:`Finished`
          (set `self.IsOpen` (not (`self.IsOpen`))))))
    (:`B`
      (goto _label :!via `Reverse`))))

(fn `Interact`
  (params (Instigator :type "Actor Object Reference"))
  (returns (Success :type Boolean))
  (`self.ToggleDoor`)
  (return true))

(fn `UserConstructionScript`)